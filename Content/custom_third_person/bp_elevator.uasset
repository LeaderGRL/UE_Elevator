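; Elevator actor that steps up or down along its own up vector when GoUp or GoDown is called.
; Both functions pass a direction to MoveToDirection, then set BisUp to record the last direction moved.
; MoveToDirection normalizes the direction, scales it by StepAmount and offsets the actor location instantly, without sweep or interpolation.
; Tick is empty, and nothing in this Blueprint calls GoUp or GoDown.
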(event EventTick
  (params (DeltaSeconds :type Float%20%28single-precision%29)))

(fn ConstructionScript)

(fn MovetoDirection
  (params (direction :type Vector))
  (Transformation|SetActorLocation (+ (* (Math|Vector|Normalize direction) (Variables|Default|GetstepAmount)) (Transformation|GetActorLocation)) false false))

(fn GoUp
  (CallFunction|MovetoDirection (Transformation|GetActorUpVector))
  (Variables|Default|SetbisUp true))

(fn GoDown
  (CallFunction|MovetoDirection (* (Transformation|GetActorUpVector) -1.0))
  (Variables|Default|SetbisUp false))